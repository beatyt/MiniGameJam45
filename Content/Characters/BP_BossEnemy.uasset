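; Boss enemy character that chases the top-down player, turns to face them every tick and fires projectiles.
; A looping timer drives a Sequence state machine through delayed ranged attack, brief speed boost and RunAway steps.
; Movement re-issues AIMoveTo toward the player after each success or failure, while RunAway's move has no destination set.
; The suggested projectile velocity is never applied, and Damage only prints the amount.
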(event Custom|AttackCycle1
  (Development|PrintString (Utilities|String|ToString(Integer) (Variables|Default|GetSequence)))
  (switch int (Variables|Default|GetSequence)
    (:0
      (CallFunction|Attack))
    (:1
      (CallFunction|Runto))
    (:2
      (CallFunction|RunAway))
    (:3
      (CallFunction|Attack)
      (Variables|Default|SetSequence 0))))

(event Custom|StartMovement
  ;[0.15 0.15 0.15 0.5] Movement
  (bind _returnvalue (Actor|GetActorOfClass "/Game/TopDown/Blueprints/BP_TopDownCharacter.BP_TopDownCharacter_C"))
  (Variables|Default|SetPlayer _returnvalue)
  (AI|AIMoveTo self "0, 0, 0" (Variables|Default|GetPlayer) 5.0 false
    (:OnSuccess
      (Utilities|FlowControl|Delay 2.0)
      (CallFunction|StartMovement))
    (:OnFail
      (Utilities|FlowControl|Delay 2.0)
      (CallFunction|StartMovement))))

(event Custom|Attack
  (bind _returnvalue (Game|GetPlayerCameraManager 0))
  (bind _returnvalue_2 (Transformation|GetActorLocation))
  (bind _player (Variables|Default|GetPlayer))
  (bind _transformcomponent (Variables|/Script/Engine.PlayerCameraManager|GetTransformComponent _returnvalue))
  (bind _returnvalue_3 (Math|Vector|GetForwardVector _transformcomponent))
  ;[0.15 0.15 0.15 0.5] Attack Sequence 1
  (Utilities|FlowControl|Delay 3.0)
  (if (<= (Transformation|GetDistanceTo _player) 6e+03)
    (bind _returnvalue_4 (Game|SpawnActorfromClass "/Game/Variant_TwinStick/Blueprints/BP_EnemyProjectile.BP_EnemyProjectile_C" (Math|Transform|MakeTransform _returnvalue_2 (Math|Rotator|FindLookatRotation _returnvalue_2 (Transformation|GetActorLocation _player))) "Undefined" "MultiplyWithRoot" 0 0))
    (Class|GameplayStatics|SuggestProjectileVelocityMovingTarget _returnvalue_2 _returnvalue_4 (* (Math|Vector|Normalize (Math|Vector|MakeVector (.x _returnvalue_3) (.y _returnvalue_3) 0.5)) 3e+03) 0.0 3.6 "None")
    (Variables|Default|SetSequence 1)))

(event Custom|Run%20To
  (bind _charactermovement (Variables|Character|GetCharacterMovement))
  ;[0.15 0.15 0.15 0.5] Sequence 2
  (Variables|/Script/Engine.CharacterMovementComponent|SetMaxWalkSpeed _charactermovement 4e+02)
  (Utilities|FlowControl|Delay 2.0)
  (Variables|/Script/Engine.CharacterMovementComponent|SetMaxWalkSpeed _charactermovement 3e+02)
  (Variables|Default|SetSequence 2))

(event Custom|LookAtU
  (bind _returnvalue (Transformation|GetActorLocation))
  (bind _player (Variables|Default|GetPlayer))
  (bind _returnvalue_2 (Transformation|GetActorLocation _player))
  (bind _returnvalue_3 (Math|Rotator|FindLookatRotation _returnvalue _returnvalue_2))
  (bind (_roll _pitch _yaw) (Math|Rotator|BreakRotator _returnvalue_3))
  (Transformation|SetActorRotation (Math|Rotator|MakeRotator _roll _pitch _yaw)))

(event Custom|Run%20Away
  (AI|AIMoveTo self "0, 0, 0" 0 5.0 false
    (:then
      (Variables|Default|SetSequence 3))))

(event EventBeginPlay
  (Utilities|Time|SetTimerbyEvent (delegate Custom|AttackCycle1) 4.0 true)
  (CallFunction|StartMovement))

(event Collision|EventActorBeginOverlap
  (params (OtherActor :type Actor%20Object%20Reference)))

(event EventTick
  (params (DeltaSeconds :type Float%20%28single-precision%29))
  (CallFunction|LookatU))

(event EventDamage
  (params (DamageAmount :type Float%20%28double-precision%29))
  (Development|PrintString (Utilities|String|ToString(Float) DamageAmount)))

(fn ConstructionScript)