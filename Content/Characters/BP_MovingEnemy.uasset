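; BP_MovingEnemy is an enemy that chases and faces the BP_TopDownCharacter and awards it XP on death.
; Tick turns it toward the player and calls StartMovement every frame, which issues AIMoveTo and also re-calls itself 0.2 seconds after success or failure.
; Damage feeds the BCHealth component and plays a sound; its OnDeath event grants XP through the player's BCXP, then sets a short lifespan.
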(event Custom|OnDeath_Event
  (CallFunction|GiveXP)
  (Actor|SetLifeSpan 0.1))

(event Custom|StartMovement
  (bind _returnvalue (Actor|GetActorOfClass "/Game/TopDown/Blueprints/BP_TopDownCharacter.BP_TopDownCharacter_C"))
  (Variables|Default|SetPlayer _returnvalue)
  (AI|AIMoveTo self "0, 0, 0" (Variables|Default|GetPlayer) 5.0 false
    (:OnSuccess
      (Utilities|FlowControl|Delay 0.2)
      (CallFunction|StartMovement))
    (:OnFail
      (Utilities|FlowControl|Delay 0.2)
      (CallFunction|StartMovement))))

(event Custom|PlaySfx
  (Audio|Components|Audio|Play (Variables|Default|GetSfx) 0.0))

(event Custom|LookAtU
  (bind _returnvalue (Transformation|GetActorLocation))
  (bind _player (Variables|Default|GetPlayer))
  (bind _returnvalue_2 (Transformation|GetActorLocation _player))
  (bind _returnvalue_3 (Math|Rotator|FindLookatRotation _returnvalue _returnvalue_2))
  (bind (_roll _pitch _yaw) (Math|Rotator|BreakRotator _returnvalue_3))
  (Transformation|SetActorRotation (Math|Rotator|MakeRotator _roll _pitch _yaw)))

(event EventBeginPlay
  (Utilities|FlowControl|Sequence
    (:then_0
      (EventDispatchers|BindEventtoOnDeath (Variables|Default|GetBCHealth) (delegate Custom|OnDeath_Event))
      (bind _returnvalue (Actor|GetActorOfClass "/Game/TopDown/Blueprints/BP_TopDownCharacter.BP_TopDownCharacter_C"))
      (Variables|Default|SetPlayer _returnvalue)
      (AI|AIMoveTo self "0, 0, 0" (Variables|Default|GetPlayer) 5.0 false))))

(event Collision|EventActorBeginOverlap
  (params (OtherActor :type Actor%20Object%20Reference)))

(event EventTick
  (params (DeltaSeconds :type Float%20%28single-precision%29))
  (CallFunction|LookatU)
  (CallFunction|StartMovement))

(event EventDamage
  (params (DamageAmount :type Float%20%28double-precision%29))
  (Default|TakeDamage (Variables|Default|GetBCHealth) DamageAmount)
  (CallFunction|PlaySfx))

(fn ConstructionScript)

(fn GiveXP
  (Default|IncreaseXP (Variables|/Game/TopDown/Blueprints/BP_TopDownCharacter.BP_TopDownCharacter_C|GetBCXP (Variables|Default|GetPlayer)) (Variables|Default|GetXP)))