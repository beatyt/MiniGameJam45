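; BP_Enemy is an enemy actor that relies on a BCHealth component for damage and death.
; On BeginPlay it binds handlers to the component's OnDamaged and OnDeath events; death prints a message and destroys the actor.
; The damage handler calls TakeDamage on the same component with zero damage, and hits on the Cylinder component only print a debug string.
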(event OnComponentHit(Cylinder)
  (params (HitComponent :type Primitive%20Component%20Object%20Reference) (OtherActor :type Actor%20Object%20Reference) (OtherComp :type Primitive%20Component%20Object%20Reference) (NormalImpulse :type Vector :default "0, 0, 0") (Hit :type Hit%20Result%20Structure%20%28by%20ref%29))
  (Development|PrintString "Ow"))

(event Custom|OnDamaged_Event
  (Default|TakeDamage (Variables|Default|GetBCHealth) 0.0))

(event Custom|OnDeath_Event
  (Development|PrintString "NOOOOOO")
  (Actor|DestroyActor))

(event EventBeginPlay
  (bind _bchealth (Variables|Default|GetBCHealth))
  (EventDispatchers|BindEventtoOnDamaged _bchealth (delegate Custom|OnDamaged_Event))
  (EventDispatchers|BindEventtoOnDeath _bchealth (delegate Custom|OnDeath_Event)))

(event Collision|EventActorBeginOverlap
  (params (OtherActor :type Actor%20Object%20Reference)))

(event EventTick
  (params (DeltaSeconds :type Float%20%28single-precision%29)))

(fn ConstructionScript)